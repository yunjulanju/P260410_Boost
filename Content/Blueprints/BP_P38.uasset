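; Player-controlled P-38 plane pawn that flies forward continuously, spins its two propellers and fires rockets.
; Tick rotates both propellers and feeds forward movement input to FloatingPawnMovement, while Pitch and Roll axes rotate the actor locally.
; Holding Boost switches max speed and propeller spin rate between normal and boost values.
; Fire spawns a BP_Rocket at the Arrow component's location, with the plane as owner and instigator.
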(event EventBeginPlay)

(event Collision|EventActorBeginOverlap
  (params (OtherActor :type Actor%20Object%20Reference)))

(event EventTick
  (params (DeltaSeconds :type Float%20%28single-precision%29))
  (Utilities|FlowControl|Sequence
    (:then_0
      (CallFunction|RotatePropeller (Variables|Default|GetR))
      (CallFunction|RotatePropeller (Variables|Default|GetL)))
    (:then_1
      (Pawn|Input|AddMovementInput (Transformation|GetActorForwardVector) (* DeltaSeconds (Variables|Speed|GetMoveSpeed)) false))))

(event Input|ActionEvents|InputActionFire
  (params (Key :type Key%20Structure :default "None"))
  (:Pressed
    (CallFunction|Fire)))

(event Input|ActionEvents|InputActionBoost
  (params (Key :type Key%20Structure :default "None"))
  (:Pressed
    (Variables|/Script/Engine.FloatingPawnMovement|SetMaxSpeed (Variables|Default|GetFloatingPawnMovement) (Variables|Speed|GetBoostSpeed))
    (Variables|Rotation|SetRotationSpeed (Variables|Rotation|GetBoostRotationSpeed)))
  (:Released
    (Variables|/Script/Engine.FloatingPawnMovement|SetMaxSpeed (Variables|Default|GetFloatingPawnMovement) (Variables|Speed|GetNormalSpeed))
    (Variables|Rotation|SetRotationSpeed (Variables|Rotation|GetNormalRotationSpeed))))

(event Input|AxisEvents|InputAxisPitch
  (params (AxisValue :type Float%20%28single-precision%29))
  (Transformation|AddActorLocalRotation (Math|Rotator|MakeRotator 0.0 (* AxisValue (Variables|Rotation|GetRotationSpeed_Body) (Utilities|Time|GetWorldDeltaSeconds)) 0.0) false false))

(event Input|AxisEvents|InputAxisRoll
  (params (AxisValue :type Float%20%28single-precision%29))
  (Transformation|AddActorLocalRotation (Math|Rotator|MakeRotator (* AxisValue (Variables|Rotation|GetRotationSpeed_Body) (Utilities|Time|GetWorldDeltaSeconds)) 0.0 0.0) false false))

(fn ConstructionScript)

(fn RotatePropeller
  (params (Target :type Scene%20Component%20Object%20Reference))
  (Transformation|AddLocalRotation Target (Math|Rotator|MakeRotator (* (Utilities|Time|GetWorldDeltaSeconds) (Variables|Rotation|GetRotationSpeed)) 0.0 0.0) false false))

(fn Fire
  (bind _self self)
  (Game|SpawnActorfromClass "/Game/Blueprints/BP_Rocket.BP_Rocket_C" (Math|Transform|MakeTransform (Transformation|GetWorldLocation (Variables|Default|GetArrow)) "0, 0, 0" "1.000000,1.000000,1.000000") "AdjustIfPossibleButAlwaysSpawn" "MultiplyWithRoot" _self _self))